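; Physics-driven ball projectile that publishes its position to a material parameter collection and caps its speed every tick.
; Events enable physics and set direction or random speed, with velocity changes gated by a short cooldown; the first hit while simulating marks it launched.
; Once launched, staying too slow or too perpendicular to X makes it blink increasingly fast, then request a replacement from the game mode and self-destruct with an explosion.
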(event OnComponentHit(CollisionSphere)
  (params (HitComponent :type Primitive%20Component%20Object%20Reference) (OtherActor :type Actor%20Object%20Reference) (OtherComp :type Primitive%20Component%20Object%20Reference) (NormalImpulse :type Vector :default "0, 0, 0") (Hit :type Hit%20Result%20Structure%20%28by%20ref%29))
  ;[0.19 0.117 0] Hit
  (if (Physics|IsSimulatingPhysics (Variables|Default|GetCollisionSphere) "None")
    (Utilities|FlowControl|DoOnce false
      (:Completed
        (Variables|Default|SetIs%20Launched%20? true)))))

(event Custom|Set%20Velocity
  (params (New%20Velocity :type Vector) (New%20Color :type Linear%20Color%20Structure))
  ;[0.16 0 0] Custom Events
  (Utilities|FlowControl|DoOnce false :!label _label
    (:Completed
      (Class|PrimitiveComponent|SetAllPhysicsLinearVelocity (Variables|Default|GetCollisionSphere) New%20Velocity false)
      (Utilities|FlowControl|Delay 0.5)
      (goto _label Reset))))

(event Custom|Set%20Movement%20Direction
  (params (New%20Direction :type Vector) (New%20Color :type Linear%20Color%20Structure))
  ;[0.16 0 0] Custom Events
  (CallFunction|SetVelocity (* (Math|Vector|Normalize New%20Direction) (Math|Float|Clamp(Float) (Math|Vector|VectorLength (Transformation|GetVelocity)) (Variables|Default|GetBall%20Min%20Speed) (Variables|Default|GetBall%20Max%20Speed))) New%20Color))

(event Custom|Enable%20Physics%20Simulation
  (bind _collisionsphere (Variables|Default|GetCollisionSphere))
  ;[0.16 0 0] Custom Events
  (Physics|SetSimulatePhysics _collisionsphere true)
  (Class|PrimitiveComponent|SetAllPhysicsLinearVelocity _collisionsphere "0, 0, 0" false))

(event Custom|Set%20Random%20Velocity
  (params (New%20Direction :type Vector) (Min%20Speed%20Ratio :type Float%20%28single-precision%29) (New%20Color :type Linear%20Color%20Structure))
  ;[0.16 0 0] Custom Events
  (CallFunction|SetVelocity (* (Math|Vector|Normalize New%20Direction) (* (Math|Random|RandomFloatinRange Min%20Speed%20Ratio 1.0) (Variables|Default|GetBall%20Max%20Speed))) New%20Color))

(event EventTick
  (params (DeltaSeconds :type Float%20%28single-precision%29))
  ;[0 0.02625 0.13] Tick
  (Variables|Default|SetDelta%20Seconds DeltaSeconds)
  (Rendering|Material|SetVectorParameterValue "/Game/Assets/Materials/Collections/ParameterCollection.ParameterCollection" "Ball Position" (Math|Conversions|ToLinearColor(Vector) (Transformation|GetActorLocation)) :!class /Script/Engine.KismetMaterialLibrary)
  (bind _returnvalue (Physics|GetPhysicsLinearVelocity (Variables|Default|GetCollisionSphere) "None"))
  (Class|PrimitiveComponent|SetAllPhysicsLinearVelocity (Variables|Default|GetCollisionSphere) (Math|Vector|ClampVectorSize _returnvalue 0.0 2e+03) false)
  (if (Variables|Default|GetIs%20Launched%20?)
    (if (or (< (Utilities|GetMovementSpeed) (Variables|Default|GetDead%20Ball%20Speed)) (< (Math|Float|Absolute(Float) (Math|Vector|DotProduct (Utilities|GetMovementDirection) "1.000000, 0,0.000000")) (Variables|Default|GetDead%20Dot%20Value)))
      (Variables|Default|SetDead%20State%20Time (+ (Variables|Default|GetDead%20State%20Time) (Variables|Default|GetDelta%20Seconds)))
      (Utilities|FlowControl|Sequence
        (:then_0
          (if (> (Variables|Default|GetDead%20State%20Time) (/ (Variables|Default|GetMin%20Dead%20Time%20To%20Auto%20Destroy) 2.0))
            (Utilities|FlowControl|Delay (Math|Float|Lerp 0.08 0.02 (Math|Float|Clamp(Float) (/ (Variables|Default|GetDead%20State%20Time) (Variables|Default|GetMin%20Dead%20Time%20To%20Auto%20Destroy)))))
            (Rendering|SetVisibility (Variables|Default|GetSphere_StaticMesh) (not (Variables|/Script/Engine.SceneComponent|GetbVisible (Variables|Default|GetSphere_StaticMesh))) true)))
        (:then_1
          (Math|Float|CompareFloat (Variables|Default|GetDead%20State%20Time) (Variables|Default|GetMin%20Dead%20Time%20To%20Auto%20Destroy)
            (:>
              (Utilities|FlowControl|DoOnce false
                (:Completed
                  (Class|BPGameModeInterface|SpawnNewBall(Message) (Game|GetGameMode))
                  (Actor|DestroyActor)))))))
      (else
        (Variables|Default|SetDead%20State%20Time 0.0)
        (Rendering|SetVisibility (Variables|Default|GetSphere_StaticMesh) true true)))))

(event EventDestroyed
  ;[1 0 0.4007] Destoyed
  (Effects|SpawnEmitteratLocation "/Game/Assets/Particles/PS_BallExplosion.PS_BallExplosion" (Transformation|GetActorLocation) (Math|Random|RandomRotator true)))

(fn ConstructionScript)