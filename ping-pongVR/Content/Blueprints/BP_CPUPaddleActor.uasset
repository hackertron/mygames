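; CPU-controlled paddle that tracks the game mode's current ball and returns it toward a destination box.
; Tick interpolates at constant speed within arena bounds while the ball moves toward +X, gating vertical tracking by a distance check, otherwise optionally recentering.
; Overlap redirects the ball to a random point in the box, optionally randomizing speed, with a one-second DoOnce cooldown and material flash.
; Construction script positions both boxes and previews the shot with an arrow.
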(event OnComponentBeginOverlap(Paddle_TriggerBox)
  (params (OverlappedComponent :type Primitive%20Component%20Object%20Reference) (OtherActor :type Actor%20Object%20Reference) (OtherComp :type Primitive%20Component%20Object%20Reference) (OtherBodyIndex :type Integer) (bFromSweep :type Boolean) (SweepResult :type Hit%20Result%20Structure%20%28by%20ref%29))
  ;[0.02575 0 0.04] Begin Overlap
  (bind _asbp_ball_projectile (Utilities|Casting|CastToBP_BallProjectile OtherActor))
  (Utilities|FlowControl|DoOnce false :!label _label
    (:Completed
      (bind _returnvalue (CallFunction|GetDirectiontoDestination _asbp_ball_projectile))
      (if (Variables|Default|GetRandom%20%20Launch%20Speed%20?)
        (Default|SetRandomVelocity _asbp_ball_projectile _returnvalue 0.5)
        (else
          (Default|SetMovementDirection _asbp_ball_projectile _returnvalue)))
      (Utilities|FlowControl|Sequence
        (:then_0
          (Utilities|FlowControl|Delay 1.0)
          (goto _label Reset))
        (:then_1
          (Timeline|Flashing%20Timeline PlayFromStart
            (:Normal
              (Rendering|Material|SetMaterial (Variables|Default|GetPaddle_StaticMesh) 0 "/Game/Assets/Materials/Instances/MI_CPUPaddle_Orange.MI_CPUPaddle_Orange")
              (Rendering|Material|SetMaterial (Variables|Default|GetPaddle_StaticMesh) 1 "/Game/Assets/Materials/Instances/MI_CPUPaddle_Yellow.MI_CPUPaddle_Yellow")
              (Rendering|Material|SetMaterial (Variables|Default|GetPaddle_StaticMesh) 2 "/Game/Assets/Materials/Instances/MI_CPUPaddle_Orange.MI_CPUPaddle_Orange"))
            (:Inverted
              (Rendering|Material|SetMaterial (Variables|Default|GetPaddle_StaticMesh) 0 "/Game/Assets/Materials/Instances/MI_CPUPaddle_Yellow.MI_CPUPaddle_Yellow")
              (Rendering|Material|SetMaterial (Variables|Default|GetPaddle_StaticMesh) 1 "/Game/Assets/Materials/Instances/MI_CPUPaddle_Orange.MI_CPUPaddle_Orange")
              (Rendering|Material|SetMaterial (Variables|Default|GetPaddle_StaticMesh) 2 "/Game/Assets/Materials/Instances/MI_CPUPaddle_Yellow.MI_CPUPaddle_Yellow"))))))))

(event EventBeginPlay
  ;[0.1 0.009139 0] begin Play
  (Variables|Default|SetPaddle%20Start%20Location (Utilities|GetPaddleLocation)))

(event EventTick
  (params (DeltaSeconds :type Float%20%28single-precision%29))
  (bind (_min _max) (Utilities|GetPaddleHorizonalBounds))
  (bind (_min_2 _max_2) (Utilities|GetPaddleVerticalBounds))
  (bind _paddle_start_location (Variables|Default|GetPaddle%20Start%20Location))
  (bind (_x _y _z) (Math|Vector|BreakVector _paddle_start_location))
  ;[0 0.006865 0.085] Tick
  (Variables|Default|SetDelta%20Seconds DeltaSeconds)
  (bind _return_value (Class|BPGameModeInterface|GetCurrentBallReference(Message) (Game|GetGameMode)))
  (bind _output_get (Variables|Default|SetCurrent%20Ball%20 _return_value))
  (Utilities|IsValid _output_get
    (:Is%20Valid
      (if (> (.X (Math|Vector|BreakVector (Transformation|GetVelocity (Variables|Default|GetCurrent%20Ball%20)))) 0.0)
        (Transformation|SetWorldLocation (Variables|Default|GetPaddle_TriggerBox) (Math|Interpolation|VInterptoConstant (Utilities|GetPaddleLocation) (Math|Vector|MakeVector _x (Math|Float|Clamp(Float) (.y (Transformation|GetActorLocation (Variables|Default|GetCurrent%20Ball%20))) _min _max) (select (|CheckifCantrackTheBallHorizontally) (Math|Float|Clamp(Float) (.z (Transformation|GetActorLocation (Variables|Default|GetCurrent%20Ball%20))) _min_2 _max_2) _z)) (Variables|Default|GetDelta%20Seconds) (Variables|Default|GetMovement%20Speed)) false false)
        (else
          (if (Variables|Default|GetAuto%20Recenter%20?) :!label _label
            (Transformation|SetWorldLocation (Variables|Default|GetPaddle_TriggerBox) (Math|Interpolation|VInterptoConstant (Utilities|GetPaddleLocation) (Variables|Default|GetPaddle%20Start%20Location) (Variables|Default|GetDelta%20Seconds) (Variables|Default|GetMovement%20Speed)) false false)))))
    (:Is%20Not%20Valid
      (goto _label))))

(fn ConstructionScript
  (bind _paddle_triggerbox (Variables|Default|GetPaddle_TriggerBox))
  (bind _ball_destination_box (Variables|Default|GetBall%20Destination%20Box))
  (bind _returnvalue (Transformation|GetWorldLocation _paddle_triggerbox))
  (bind _returnvalue_2 (Transformation|GetWorldLocation _ball_destination_box))
  (bind _returnvalue_3 (- _returnvalue_2 _returnvalue))
  (Transformation|SetRelativeTransform (Variables|Default|GetPaddle_TriggerBox) (Variables|Default|GetPaddle%20Transform) false false)
  (Transformation|SetRelativeTransform (Variables|Default|GetBall%20Destination%20Box) (Variables|Default|GetBall%20Destination%20Box%20Transform) false false)
  (Transformation|SetWorldLocationAndRotation (Variables|Default|GetArrow) _returnvalue (Math|Conversions|RotationFromXVector _returnvalue_3) false false)
  (Transformation|SetWorldScale3D (Variables|Default|GetArrow) (Math|Vector|MakeVector (/ (Math|Vector|VectorLength _returnvalue_3) 1e+02) 2.0 2.0)))

(fn GetDirectiontoDestination
  (params (Ball :type Actor%20Object%20Reference))
  (bind _ball_destination_box (Variables|Default|GetBall%20Destination%20Box))
  (bind (_origin _boxextent) (Collision|GetComponentBounds _ball_destination_box))
  (return (- (Math|Random|RandomPointinBoundingBox _origin _boxextent) (Transformation|GetActorLocation Ball))))