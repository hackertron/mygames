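; Game mode for a Player-versus-CPU ball game that tracks match state, both scores and the current ball.
; It implements a GameMode interface, forwarding new-game, ball-spawn, score and hit-message updates to a registered MainGame reference.
; Spawning a new ball destroys the current one before asking MainGame for its replacement.
; Getters expose the ball, MainGame reference and match-started flag to other Blueprints.
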(event EventSetMainGameReference
  (params (Main%20Game :type BP%20Main%20Game%20Actor%20Object%20Reference))
  ;[0.115 0 0] GameMode Interface Events
  (Variables|Default|SetMain%20Game%20Reference Main%20Game))

(event EventUpdateScore
  (params (Target :type Enum_GoalOwner%20Enum))
  ;[0.115 0 0] GameMode Interface Events
  (bind _main_game_reference (Variables|Default|GetMain%20Game%20Reference)
    (:then
      (Utilities|FlowControl|Sequence
        (:then_0
          (switch Utilities|FlowControl|Switch|SwitchonEnum_GoalOwner Target
            (:NewEnumerator0
              (Math|Integer|IncrementInt (Variables|Default|GetPlayer%20Score)))
            (:NewEnumerator1
              (Math|Integer|IncrementInt (Variables|Default|GetCPU%20Score)))))
        (:then_1
          (Default|OnScoreUpdated _main_game_reference (Variables|Default|GetPlayer%20Score) (Variables|Default|GetCPU%20Score)))))
    (:else)))

(event EventStartNewGame
  ;[0.115 0 0] GameMode Interface Events
  (bind _main_game_reference (Variables|Default|GetMain%20Game%20Reference)
    (:then
      (Default|StartNewGameEvent _main_game_reference))
    (:else)))

(event EventStartMatch
  ;[0.115 0 0] GameMode Interface Events
  (Variables|Default|SetMatch%20Started%20? true)
  (bind _main_game_reference (Variables|Default|GetMain%20Game%20Reference)
    (:then
      (Default|HideHitMessage _main_game_reference))
    (:else)))

(event EventFinishMatch
  ;[0.115 0 0] GameMode Interface Events
  (Variables|Default|SetMatch%20Started%20? false))

(event EventSpawnNewBall
  ;[0.115 0 0] GameMode Interface Events
  (Utilities|FlowControl|Sequence
    (:then_0
      (bind _current_ball_reference (Variables|Default|GetCurrent%20Ball%20Reference)
        (:then
          (Actor|DestroyActor _current_ball_reference))
        (:else)))
    (:then_1
      (bind _main_game_reference (Variables|Default|GetMain%20Game%20Reference)
        (:then
          (Default|SpawnNewBallEvent _main_game_reference))
        (:else)))))

(event EventSetCurrentBallReference
  (params (New%20Ball :type BP%20Ball%20Projectile%20Object%20Reference))
  ;[0.115 0 0] GameMode Interface Events
  (Variables|Default|SetCurrent%20Ball%20Reference New%20Ball))

(fn ConstructionScript)

(fn GetCurrentBallReference
  (return (Variables|Default|GetCurrent%20Ball%20Reference)))

(fn GetMainGameReference
  (return (Variables|Default|GetMain%20Game%20Reference)))

(fn HasMatchStarted
  (return (Variables|Default|GetMatch%20Started%20?)))