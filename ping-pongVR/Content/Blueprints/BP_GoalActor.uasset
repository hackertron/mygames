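; Goal actor that detects the ball, credits a point to the side opposite its owner and requests a new ball.
; On trigger overlap, a DoOnce gate blocks repeat scoring while the ball is destroyed and the game mode is messaged.
; A timeline then animates two sphere radii around the goal through a material parameter collection, resetting them before re-arming.
; The construction script builds tinted dynamic materials for frame and grid.
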(event OnComponentBeginOverlap(Goal_TriggerBox)
  (params (OverlappedComponent :type Primitive%20Component%20Object%20Reference) (OtherActor :type Actor%20Object%20Reference) (OtherComp :type Primitive%20Component%20Object%20Reference) (OtherBodyIndex :type Integer) (bFromSweep :type Boolean) (SweepResult :type Hit%20Result%20Structure%20%28by%20ref%29))
  ;[0.06615 0.09525 0.24] Begin Overlap
  (bind _asbp_ball_projectile (Utilities|Casting|CastToBP_BallProjectile OtherActor))
  (Utilities|FlowControl|DoOnce false :!label _label
    (:Completed
      (Rendering|Material|SetVectorParameterValue "/Game/Assets/Materials/Collections/ParameterCollection.ParameterCollection" "Animation Center" (Math|Conversions|ToLinearColor(Vector) (Transformation|GetWorldLocation (Variables|Default|GetGrid_StaticMesh))) :!class /Script/Engine.KismetMaterialLibrary)
      (Actor|DestroyActor _asbp_ball_projectile)
      (Class|BPGameModeInterface|UpdateScore(Message) (Game|GetGameMode) (Utilities|Select :Index (Variables|Default|GetGoal%20Owner) :NewEnumerator0 "NewEnumerator1" :NewEnumerator1 "NewEnumerator0"))
      (Utilities|FlowControl|Delay 0.2)
      (bind (_direction _animation_1_alpha _animation_2_alpha) (Timeline|Timeline_0 PlayFromStart)
        (:Update
          (Rendering|Material|SetScalarParameterValue "/Game/Assets/Materials/Collections/ParameterCollection.ParameterCollection" "Goal Sphere Radius 1" (Math|Float|Lerp 5e+01 6e+02 _animation_1_alpha) :!class /Script/Engine.KismetMaterialLibrary)
          (Rendering|Material|SetScalarParameterValue "/Game/Assets/Materials/Collections/ParameterCollection.ParameterCollection" "Goal Sphere Radius 2" (Math|Float|Lerp 0.0 6e+02 _animation_2_alpha) :!class /Script/Engine.KismetMaterialLibrary))
        (:Finished
          (Class|BPGameModeInterface|SpawnNewBall(Message) (Game|GetGameMode))
          (Rendering|Material|SetScalarParameterValue "/Game/Assets/Materials/Collections/ParameterCollection.ParameterCollection" "Goal Sphere Radius 1" 0.0 :!class /Script/Engine.KismetMaterialLibrary)
          (Rendering|Material|SetScalarParameterValue "/Game/Assets/Materials/Collections/ParameterCollection.ParameterCollection" "Goal Sphere Radius 2" 0.0 :!class /Script/Engine.KismetMaterialLibrary)
          (goto _label Reset))))))

(fn ConstructionScript
  (Utilities|FlowControl|Sequence
    (:then_0
      (bind _returnvalue (Rendering|Material|CreateDynamicMaterialInstance "/Game/Assets/Materials/M_Frame_Master.M_Frame_Master" :!class /Script/Engine.KismetMaterialLibrary))
      (bind _output_get (LocalVariables|SetTemp%20Material%20Instance _returnvalue))
      (Rendering|Material|SetVectorParameterValue _output_get "Color" (Variables|Default|GetGoal%20Color) :!class /Script/Engine.MaterialInstanceDynamic)
      (Rendering|Material|SetMaterial (Variables|Default|GetFrame_StaticMesh) 0 (LocalVariables|GetTemp%20Material%20Instance)))
    (:then_1
      (bind _returnvalue_2 (Rendering|Material|CreateDynamicMaterialInstance "/Game/Assets/Materials/M_Goal_master.M_Goal_master" :!class /Script/Engine.KismetMaterialLibrary))
      (bind _output_get_2 (LocalVariables|SetTemp%20Material%20Instance _returnvalue_2))
      (Rendering|Material|SetVectorParameterValue _output_get_2 "Color" (Variables|Default|GetGoal%20Color) :!class /Script/Engine.MaterialInstanceDynamic)
      (Rendering|Material|SetScalarParameterValue (LocalVariables|GetTemp%20Material%20Instance) "Grid Scale" (Variables|Default|GetGrid%20Scale) :!class /Script/Engine.MaterialInstanceDynamic)
      (Rendering|Material|SetMaterial (Variables|Default|GetGrid_StaticMesh) 0 (LocalVariables|GetTemp%20Material%20Instance)))))