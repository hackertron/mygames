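; Main game actor for a player-versus-CPU paddle-and-ball game, registering itself with the game mode and running round start, ball launch and in-world UI.
; A new game updates start messages, spawns a ball that a timeline moves to its target before enabling physics, then animates paddle dissolve through a Material Parameter Collection.
; Score and message events update 3D widget components.
; Ball hits spawn impact particles, debounced by a resetting DoOnce.
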(event Custom|Spawn%20New%20Ball%20Event
  ;[0.15 0 0] Custom Events
  (Components|Activation|Activate (Variables|Default|GetSpawner_ParticleSystem) true)
  (Utilities|FlowControl|Delay 0.2)
  (bind _returnvalue (Game|SpawnActorfromClass "/Game/Blueprints/BP_BallProjectile.BP_BallProjectile_C" (Math|Transform|MakeTransform (Transformation|GetWorldLocation (Variables|Default|GetBallSpawnPoint)) "0,0.000000, 0") "Undefined" 0 3e+02 2.5e+03 2e+02 2.0 0.15))
  (Class|BPGameModeInterface|SetCurrentBallReference(Message) (Game|GetGameMode) _returnvalue)
  (bind _lerp_alpha (Timeline|Timeline_0 PlayFromStart)
    (:Update
      (bind _return_value (Class|BPGameModeInterface|GetCurrentBallReference(Message) (Game|GetGameMode)))
      (Transformation|SetActorLocation _return_value (Math|Vector|Lerp(Vector) (Transformation|GetWorldLocation (Variables|Default|GetBallSpawnPoint)) (Transformation|GetWorldLocation (Variables|Default|GetBallTargetPoint)) _lerp_alpha) false false))
    (:Finished
      (Components|Activation|Deactivate (Variables|Default|GetSpawner_ParticleSystem))
      (bind _return_value_2 (Class|BPGameModeInterface|GetCurrentBallReference(Message) (Game|GetGameMode)))
      (Default|EnablePhysicsSimulation _return_value_2))))

(event Custom|Play%20Paddles%20Animation
  ;[0.15 0 0] Custom Events
  (bind _lerp_alpha (Timeline|Paddles%20Dissolve%20Animation%20Timeline PlayFromStart)
    (:Update
      (Rendering|Material|SetScalarParameterValue "/Game/Assets/Materials/Collections/ParameterCollection.ParameterCollection" "Paddles Dissolve Amout" (Math|Float|Lerp 0.0 1.0 _lerp_alpha) :!class /Script/Engine.KismetMaterialLibrary))))

(event Custom|Show%20Hit%20Message
  ;[0.15 0 0] Custom Events
  (bind _start_message (Utilities|GetStartMessageWidgetObject)
    (:Is%20Valid
      (Default|SetHitMessageActive _start_message true))))

(event Custom|Hide%20trigger%20Message
  ;[0.15 0 0] Custom Events
  (bind _start_message (Utilities|GetStartMessageWidgetObject)
    (:Is%20Valid
      (Default|HideTriggerMessageText _start_message))))

(event Custom|Reset%20Hit%20Detection
  ;[0 0.04653 0.225] Hit
  (Utilities|FlowControl|DoOnce false) ; enters at Reset
)

(event Custom|On%20Score%20Updated
  (params (Player%20Score :type Integer) (CPU%20Score :type Integer))
  ;[0.15 0 0] Custom Events
  (bind _game_hud (Utilities|GetGameHUDWidgetObject)
    (:Is%20Valid
      (Default|UpdateScoresText _game_hud Player%20Score CPU%20Score))))

(event Custom|Start%20New%20Game%20Event
  ;[0.15 0 0] Custom Events
  (CallFunction|HideTriggerMessage)
  (CallFunction|ShowHitMessage)
  (Utilities|FlowControl|Delay 3.5)
  (CallFunction|SpawnNewBallEvent)
  (Utilities|FlowControl|Delay 0.5)
  (CallFunction|PlayPaddlesAnimation))

(event Custom|Hide%20Hit%20Message
  ;[0.15 0 0] Custom Events
  (bind _start_message (Utilities|GetStartMessageWidgetObject)
    (:Is%20Valid
      (Default|SetHitMessageActive _start_message false))))

(event EventBeginPlay
  ;[0.195 0.1474 0] Begin Play
  (Rendering|Material|SetScalarParameterValue "/Game/Assets/Materials/Collections/ParameterCollection.ParameterCollection" "Paddles Dissolve Amout" 0.0 :!class /Script/Engine.KismetMaterialLibrary)
  (Class|BPGameModeInterface|SetMainGameReference(Message) (Game|GetGameMode) self))

(event Collision|EventHit
  (params (MyComp :type Primitive%20Component%20Object%20Reference) (Other :type Actor%20Object%20Reference) (OtherComp :type Primitive%20Component%20Object%20Reference) (bSelfMoved :type Boolean) (HitLocation :type Vector :default "0, 0, 0") (HitNormal :type Vector :default "0, 0, 0") (NormalImpulse :type Vector :default "0, 0, 0") (Hit :type Hit%20Result%20Structure%20%28by%20ref%29))
  (bind (_bblockinghit _binitialoverlap _time _location _impactpoint _normal) (Collision|BreakHitResult Hit))
  ;[0 0.04653 0.225] Hit
  (Utilities|Casting|CastToBP_BallProjectile Other)
  (Utilities|FlowControl|DoOnce false
    (:Completed
      (Effects|SpawnEmitteratLocation "/Game/Assets/Particles/PS_BallCollisionImpact.PS_BallCollisionImpact" (+ _location (* _normal 5.0)) (Math|Rotator|MakeRotfromX _normal))
      (Utilities|FlowControl|Delay 0.05)
      (CallFunction|ResetHitDetection))))

(fn ConstructionScript)