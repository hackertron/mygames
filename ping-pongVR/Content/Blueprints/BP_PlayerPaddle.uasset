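; BP_PlayerPaddle is a motion-controller paddle that the player uses to hit BP_BallProjectile balls.
; SetHand assigns the MotionController to the left or right hand from an index.
; A ball hit tells the game mode to start the match if it has not already started.
; It also plays a short force-feedback pulse on that hand's side, scaled by ball speed relative to its maximum.
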(event Custom|Set%20Hand
  (params (Hand%20Index :type Integer))
  ;[0.1 0 0] custom Events
  (Variables|/Script/HeadMountedDisplay.MotionControllerComponent|SetHand (Variables|Default|GetMotionController) (Utilities|Select :Index Hand%20Index :Option%200 "Left" :Option%201 "Right")))

(event Collision|EventHit
  (params (MyComp :type Primitive%20Component%20Object%20Reference) (Other :type Actor%20Object%20Reference) (OtherComp :type Primitive%20Component%20Object%20Reference) (bSelfMoved :type Boolean) (HitLocation :type Vector :default "0, 0, 0") (HitNormal :type Vector :default "0, 0, 0") (NormalImpulse :type Vector :default "0, 0, 0") (Hit :type Hit%20Result%20Structure%20%28by%20ref%29))
  (bind _returnvalue (Game|GetGameMode))
  (bind _motioncontroller (Variables|Default|GetMotionController))
  (bind _hand (Variables|/Script/HeadMountedDisplay.MotionControllerComponent|GetHand _motioncontroller))
  (bind _returnvalue_2 (Utilities|Enum|Equal(Enum) _hand "Left"))
  (bind _returnvalue_3 (not _returnvalue_2))
  ;[0.06215 0 0.21] Hit
  (bind _asbp_ball_projectile (Utilities|Casting|CastToBP_BallProjectile Other))
  (bind _return_value (Class|BPGameModeInterface|HasMatchStarted(Message) _returnvalue))
  (if (not _return_value)
    (Class|BPGameModeInterface|StartMatch(Message) _returnvalue))
  (Game|Feedback|PlayDynamicForceFeedback (Game|GetPlayerController 0) (/ (Math|Vector|VectorLength (Transformation|GetVelocity _asbp_ball_projectile)) (Variables|/Game/Blueprints/BP_BallProjectile.BP_BallProjectile_C|GetBall%20Max%20Speed _asbp_ball_projectile)) 0.1 _returnvalue_2 _returnvalue_2 _returnvalue_3 _returnvalue_3))

(fn ConstructionScript)