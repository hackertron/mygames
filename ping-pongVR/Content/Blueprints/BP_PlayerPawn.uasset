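; BP_PlayerPawn is the VR player pawn, possessed by the first player controller on BeginPlay when a headset is connected.
; On BeginPlay it also spawns two BP_PlayerPaddle actors, assigns each a hand and attaches them to itself.
; Each tick it writes the player's base location and headset height to a material parameter collection, making both available to materials.
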(event EventBeginPlay
  ;[0.095 0 0] Begin Play
  (Utilities|FlowControl|Sequence
    (:then_0
      (if (Class|HeadMountedDisplayFunctionLibrary|IsHeadMountedDisplayConnected)
        (Pawn|Possess (Game|GetPlayerController 0) self)))
    (:then_1
      (for _index (range 0 1)
        (bind _returnvalue (Game|SpawnActorfromClass "/Game/Blueprints/BP_PlayerPaddle.BP_PlayerPaddle_C" (Math|Transform|MakeTransform "0.000000, 0,0.000000" "0, 0, 0" "1,1,1") "Undefined" 0 0))
        (Default|SetHand _returnvalue _index)
        (Transformation|AttachActorToActor _returnvalue self "None" "SnapToTarget" "SnapToTarget" "KeepWorld" true)))))

(event EventTick
  (params (DeltaSeconds :type Float%20%28single-precision%29))
  ;[0 0.04656 0.14] Tick
  (Rendering|Material|SetVectorParameterValue "/Game/Assets/Materials/Collections/ParameterCollection.ParameterCollection" "Player Base Location" (Math|Conversions|ToLinearColor(Vector) (|GetPlayerBaseLocation)) :!class /Script/Engine.KismetMaterialLibrary)
  (Rendering|Material|SetScalarParameterValue "/Game/Assets/Materials/Collections/ParameterCollection.ParameterCollection" "Player Height" (.z (.DevicePosition (Class|HeadMountedDisplayFunctionLibrary|GetOrientationandPosition))) :!class /Script/Engine.KismetMaterialLibrary))

(fn ConstructionScript)