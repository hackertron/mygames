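; BP_MeshActor is a shape actor that turns its static mesh into a procedural mesh with collision at runtime.
; The construction script sets the mesh from a Shape enum (sphere, cube, cylinder, cone) or a valid override.
; BeginPlay copies that mesh into the ProceduralMesh component, then destroys the StaticMesh component.
; Randomly spawned instances also get a random rotation and uniform scale, plus an upward velocity impulse.
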(event EventBeginPlay
  ;[0.36 0 0] Begin Play
  (Components|StaticMesh|SetStaticMesh (Variables|Default|GetStaticMesh) (CallFunction|GetStaticMeshbyShapeType))
  (Transformation|SetRelativeTransform (Variables|Default|GetProceduralMesh) (Transformation|GetRelativeTransform (Variables|Default|GetStaticMesh)) false false)
  (Class|KismetProceduralMeshLibrary|CopyProceduralMeshfromStaticMeshComponent (Variables|Default|GetStaticMesh) 0 (Variables|Default|GetProceduralMesh) true)
  (Components|DestroyComponent (Variables|Default|GetStaticMesh))
  (if (Variables|Default|GetIs%20Randomly%20Spawned%20?)
    (Transformation|SetRelativeTransform (Variables|Default|GetProceduralMesh) (Math|Transform|MakeTransform (Variables|/Script/Engine.SceneComponent|GetRelativeLocation (Variables|Default|GetProceduralMesh)) (Math|Random|RandomRotator true) (Math|Conversions|ToVector(Float) (Math|Random|RandomFloatinRange 0.4 0.65))) false false)
    (Physics|AddImpulse (Variables|Default|GetProceduralMesh) "0, 0,900.000000" "None" true)))

(fn ConstructionScript
  (Components|StaticMesh|SetStaticMesh (Variables|Default|GetStaticMesh) (CallFunction|GetStaticMeshbyShapeType)))

(fn GetStaticMeshbyShapeType
  (return (select (Utilities|IsValid (Variables|Default|GetStatic%20Mesh%20Override)) (Variables|Default|GetStatic%20Mesh%20Override) (Utilities|Select :Index (Variables|Default|GetShape) :NewEnumerator0 "/Game/Assets/Meshes/Sphere.Sphere" :NewEnumerator1 "/Game/Assets/Meshes/Cube.Cube" :NewEnumerator2 "/Game/Assets/Meshes/Cylinder.Cylinder" :NewEnumerator3 "/Game/Assets/Meshes/Cone.Cone"))))