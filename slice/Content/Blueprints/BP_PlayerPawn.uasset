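; Player pawn that equips the player with hand-bound blade actors for slicing.
; On Begin Play, it spawns a BP_BladeActor for the left hand, the right hand or both, according to ActiveControllers.
; Each blade receives the pawn's double-edged and minimum slicing velocity settings at spawn, then SetupController assigns its hand with the pawn's DefaultSceneRoot as parent.
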(event EventBeginPlay
  ;[0.36 0 0] Begin Play
  (switch Utilities|FlowControl|Switch|SwitchonEnum_ActiveControllers (Variables|Default|GetActive%20Controllers)
    (:NewEnumerator0
      (bind _returnvalue (Game|SpawnActorfromClass "/Game/Blueprints/BP_BladeActor.BP_BladeActor_C" (Math|Transform|MakeTransform "0, 0, 0" "0, 0, 0" "1,1,1") "Undefined" 0 (Variables|Default|GetIs%20Double%20Edged%20Sword%20) (Variables|Default|GetMin%20Velocity%20To%20Perform%20Slicing) :!label _label))
      (Default|SetupController _returnvalue (Variables|Default|GetDefaultSceneRoot) (select (Utilities|Enum|Equal(Enum) (Variables|Default|GetActive%20Controllers) "NewEnumerator0") "Left" "Right")))
    (:NewEnumerator1
      (goto _label))
    (:NewEnumerator2
      (for _index (range 0 1)
        (bind _returnvalue_2 (Game|SpawnActorfromClass "/Game/Blueprints/BP_BladeActor.BP_BladeActor_C" (Math|Transform|MakeTransform "0, 0, 0" "0, 0, 0" "1,1,1.000000") "Undefined" 0 (Variables|Default|GetIs%20Double%20Edged%20Sword%20) (Variables|Default|GetMin%20Velocity%20To%20Perform%20Slicing)))
        (Default|SetupController _returnvalue_2 (Variables|Default|GetDefaultSceneRoot) (Utilities|Select :Index _index :Option%200 "Left" :Option%201 "Right"))))))

(fn ConstructionScript)